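; BP_Coin_1 is a collectable coin placed in levels that the player picks up by touching it.
; When the Coin component's overlap begins, it casts the other actor to BP_LevelDesign_SUM_Character, increments that character's Coins count and destroys itself.
; The coin writes to the character's variable directly, and overlaps from any other actor type are ignored.
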(event OnComponentBeginOverlap(Coin)
  (params (OverlappedComponent :type Primitive%20Component%20Object%20Reference) (OtherActor :type Actor%20Object%20Reference) (OtherComp :type Primitive%20Component%20Object%20Reference) (OtherBodyIndex :type Integer) (bFromSweep :type Boolean) (SweepResult :type Hit%20Result%20Structure%20%28by%20ref%29))
  (bind _asbp_level_design_sum_character (Utilities|Casting|CastToBP_LevelDesign_SUM_Character OtherActor))
  (bind _result (Math|Integer|IncrementInt (Variables|/Game/0_LevelDesign_BPs/Blueprints/0_Player/BP_LevelDesign_SUM_Character.BP_LevelDesign_SUM_Character_C|GetCoins _asbp_level_design_sum_character))
    (:%20%20
      (Variables|/Game/0_LevelDesign_BPs/Blueprints/0_Player/BP_LevelDesign_SUM_Character.BP_LevelDesign_SUM_Character_C|SetCoins _asbp_level_design_sum_character _result)
      (Actor|DestroyActor))))

(event EventBeginPlay
  (|CallParentFunction) ; This node is disabled and will not be called.\nDrag off pins to build functionality.
)

(event Collision|EventActorBeginOverlap
  (params (OtherActor :type Actor%20Object%20Reference))
  (|CallParentFunction OtherActor) ; This node is disabled and will not be called.\nDrag off pins to build functionality.
)

(event EventTick
  (params (DeltaSeconds :type Float%20%28single-precision%29))
  (|CallParentFunction DeltaSeconds) ; This node is disabled and will not be called.\nDrag off pins to build functionality.
)

(fn ConstructionScript
  (|CallParentFunction))