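; BP_KeyBlue is a collectable blue key pickup for the level design character.
; When its Key component is overlapped, it casts the other actor to BP_LevelDesign_SUM_Character, increments that character's BlueKeys count and calls KeyInventory.
; It then prints the new count to screen and destroys itself.
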(event OnComponentBeginOverlap(Key)
  (params (OverlappedComponent :type Primitive%20Component%20Object%20Reference) (OtherActor :type Actor%20Object%20Reference) (OtherComp :type Primitive%20Component%20Object%20Reference) (OtherBodyIndex :type Integer) (bFromSweep :type Boolean) (SweepResult :type Hit%20Result%20Structure%20%28by%20ref%29))
  (bind _asbp_level_design_sum_character (Utilities|Casting|CastToBP_LevelDesign_SUM_Character OtherActor))
  (bind _output_get (Variables|/Game/0_LevelDesign_BPs/Blueprints/0_Player/BP_LevelDesign_SUM_Character.BP_LevelDesign_SUM_Character_C|SetBlueKeys _asbp_level_design_sum_character (+ (Variables|/Game/0_LevelDesign_BPs/Blueprints/0_Player/BP_LevelDesign_SUM_Character.BP_LevelDesign_SUM_Character_C|GetBlueKeys _asbp_level_design_sum_character) 1)))
  (Default|KeyInventory _asbp_level_design_sum_character)
  (Development|PrintString (Utilities|String|ToString(Integer) _output_get))
  (Actor|DestroyActor))

(event EventBeginPlay
  (|CallParentFunction) ; This node is disabled and will not be called.\nDrag off pins to build functionality.
)

(event Collision|EventActorBeginOverlap
  (params (OtherActor :type Actor%20Object%20Reference))
  (|CallParentFunction OtherActor) ; This node is disabled and will not be called.\nDrag off pins to build functionality.
)

(event EventTick
  (params (DeltaSeconds :type Float%20%28single-precision%29))
  (|CallParentFunction DeltaSeconds) ; This node is disabled and will not be called.\nDrag off pins to build functionality.
)

(fn ConstructionScript
  (|CallParentFunction))