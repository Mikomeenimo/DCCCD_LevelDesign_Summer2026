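; BP_DoorBlue is a level-design sliding door that can require a blue key.
; Entering its box plays a timeline lerping the door to EndPoint if Unlocked; otherwise, with RequireBlueKey set and a key available, it unlocks, consumes one and refreshes the key inventory.
; Begin overlap casts to BP_LevelDesign_SUM_Character, while end overlap casts to BP_ThirdPersonCharacter before reversing the timeline.
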(event OnComponentBeginOverlap(Box)
  (params (OverlappedComponent :type Primitive%20Component%20Object%20Reference) (OtherActor :type Actor%20Object%20Reference) (OtherComp :type Primitive%20Component%20Object%20Reference) (OtherBodyIndex :type Integer) (bFromSweep :type Boolean) (SweepResult :type Hit%20Result%20Structure%20%28by%20ref%29))
  (bind _asbp_level_design_sum_character (Utilities|Casting|CastToBP_LevelDesign_SUM_Character OtherActor))
  (if (Variables|Default|GetUnlocked)
    (bind _alpha (Timeline|Timeline Play)
      (:Update
        (Transformation|SetRelativeLocation (Variables|Default|GetDoor) (Math|Vector|Lerp(Vector) (Variables|Default|GetStartingPosition) (Variables|/Script/Engine.SceneComponent|GetRelativeLocation (Variables|Default|GetEndPoint)) _alpha) false false)))
    (elif (Variables|Default|GetRequireBlueKey)
      (bind _open (Default|CanOpenBlueDoor _asbp_level_design_sum_character))
      (if _open
        (Variables|Default|SetUnlocked true)
        (Math|Integer|DecrementInt (Variables|/Game/0_LevelDesign_BPs/Blueprints/0_Player/BP_LevelDesign_SUM_Character.BP_LevelDesign_SUM_Character_C|GetBlueKeys _asbp_level_design_sum_character)
          (:%20%20
            (Default|KeyInventory _asbp_level_design_sum_character)
            (Timeline|Timeline Play)))))))

(event OnComponentEndOverlap(Box)
  (params (OverlappedComponent :type Primitive%20Component%20Object%20Reference) (OtherActor :type Actor%20Object%20Reference) (OtherComp :type Primitive%20Component%20Object%20Reference) (OtherBodyIndex :type Integer))
  (Utilities|Casting|CastToBP_ThirdPersonCharacter OtherActor)
  (bind _alpha (Timeline|Timeline Reverse)
    (:Update
      (Transformation|SetRelativeLocation (Variables|Default|GetDoor) (Math|Vector|Lerp(Vector) (Variables|Default|GetStartingPosition) (Variables|/Script/Engine.SceneComponent|GetRelativeLocation (Variables|Default|GetEndPoint)) _alpha) false false))))

(event EventBeginPlay
  (|CallParentFunction) ; This node is disabled and will not be called.\nDrag off pins to build functionality.
)

(event Collision|EventActorBeginOverlap
  (params (OtherActor :type Actor%20Object%20Reference)))

(event EventTick
  (params (DeltaSeconds :type Float%20%28single-precision%29)))

(fn ConstructionScript
  (|CallParentFunction))