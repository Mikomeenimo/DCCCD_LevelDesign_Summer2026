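; Player character Blueprint for a level-design project that tracks collected keys and creates the HUD.
; On BeginPlay it creates the W_HUD widget and adds it to the viewport.
; CanOpenBlueDoor reports whether at least one blue key is held, and KeyInventory swaps the BlueKey material between emissive blue and a basic material from that count.
; A similar red key material branch exists but is disconnected and never runs.
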(event EventBeginPlay
  (bind _returnvalue (UserInterface|CreateWidget "/Game/0_LevelDesign_BPs/Blueprints/0_Player/W_HUD.W_HUD_C"))
  (bind _output_get (Variables|Default|SetHUD _returnvalue))
  (UserInterface|Viewport|AddtoViewport _output_get 0))

(fn ConstructionScript
  (|CallParentFunction))

(fn CanOpenBlueDoor
  (Utilities|FlowControl|Sequence
    (:then_0
      (return (>= (Variables|Default|GetBlueKeys) 1)))))

(fn KeyInventory
  (Utilities|FlowControl|Sequence
    (:then_0
      (if (> (Variables|Default|GetBlueKeys) 0)
        (Rendering|Material|SetMaterial (Variables|Default|GetBlueKey) 0 "/Game/0_LevelDesign_BPs/Visuals/Materials/M_EmissiveBlue.M_EmissiveBlue")
        (else
          (Rendering|Material|SetMaterial (Variables|Default|GetBlueKey) 0 "/Engine/BasicShapes/BasicShapeMaterial_Inst.BasicShapeMaterial_Inst"))))))